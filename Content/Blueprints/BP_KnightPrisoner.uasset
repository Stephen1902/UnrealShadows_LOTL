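; BP_KnightPrisoner is a prisoner character that grants XP once when interacted with, then cheers.
; It plays a non-looping idle animation on BeginPlay.
; While CanGiveXP is set, Interact adds EarnedXP to the instigator's US_PlayerState, then CharacterCheer loops the cheer animation and clears the flag.
; CanInteract always returns false, and AddIKGoals is an empty stub.
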(event `self.ReceiveBeginPlay`
  (`SkeletalMeshComponent.PlayAnimation` (`self.SkeletalMesh`) (`self.MontageIdle`) false))

(event `CharacterCheer`
  (`SkeletalMeshComponent.PlayAnimation` (`self.SkeletalMesh`) (`self.MontageCheer`) true)
  (set `self.CanGiveXP` false))

(event `self.Interact`
  (params (CharacterInstigator :type "US_PlayerCharacter Object Reference"))
  (`KismetSystemLibrary.PrintString` "Interacting")
  (if (`self.CanGiveXP`)
    (bind _asus_player_state (cast `US_PlayerState` (`Pawn.PlayerState` CharacterInstigator)))
    (`US_PlayerState.AddXp` _asus_player_state (`self.EarnedXP`))
    (`self.CharacterCheer`)))

(fn `AddIKGoals`
  (returns (OutGoals :type "Map of Name to IKRigGoal Structure"))
  (return))

(fn `CanInteract`
  (params (CharacterInstigator :type "US_PlayerCharacter Object Reference"))
  (returns (ReturnValue :type Boolean))
  (return false))

(fn `UserConstructionScript`)